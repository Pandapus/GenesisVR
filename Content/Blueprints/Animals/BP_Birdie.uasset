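; Bird actor that flies along the spline of a referenced BirdieSplineRef actor while looping its BS_Birdie animation.
; BeginPlay places it at the first spline point.
; Tick advances the distance at a constant speed and sets world location and yaw from the spline, with no wrap-around at the end.
; Timeline, duration and start-offset logic is left unused.
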(event `self.ReceiveBeginPlay`
  (`self.K2_SetActorLocationAndRotation` (`SplineComponent.GetLocationAtSplinePoint` (`/Game/Blueprints/Animals/BP_BirdieSplinePath.Spline` (`self.BirdieSplineRef`)) 0 "World"))
  (`SkeletalMeshComponent.PlayAnimation` (`self.Birdie`) "/Game/Blueprints/Animals/BS_Birdie.BS_Birdie" true))

(event `self.ReceiveTick`
  (params (DeltaSeconds :type "Float (single-precision)"))
  (bind (_returnvalue_roll _returnvalue_pitch _returnvalue_yaw) (`KismetMathLibrary.BreakRotator` (`SplineComponent.GetRotationAtDistanceAlongSpline` (`/Game/Blueprints/Animals/BP_BirdieSplinePath.Spline` (`self.BirdieSplineRef`)) (`self.DistenceAlongSpline`) "World")))
  (bind (_returnvalue_x _returnvalue_y _returnvalue_z) (`KismetMathLibrary.BreakVector` (`SplineComponent.GetLocationAtDistanceAlongSpline` (`/Game/Blueprints/Animals/BP_BirdieSplinePath.Spline` (`self.BirdieSplineRef`)) (`self.DistenceAlongSpline`) "World")))
  (set `self.DistenceAlongSpline` (+ (* DeltaSeconds 50.0) (`self.DistenceAlongSpline`)))
  (`self.K2_SetActorLocationAndRotation` (`KismetMathLibrary.MakeVector` _returnvalue_x _returnvalue_y _returnvalue_z) (`KismetMathLibrary.MakeRotator` 0.0 0.0 _returnvalue_yaw)))

(fn `UserConstructionScript`)