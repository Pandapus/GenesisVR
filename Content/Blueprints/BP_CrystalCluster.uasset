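; BP_CrystalCluster is a group of four crystals and a sphere that glows and plays a sound when activated.
; On BeginPlay it applies its Color to the meshes' emissive color and the point light, and assigns SoundSlot to the audio component.
; Activate plays the audio and restarts the EmissionCycle timeline, which drives emissive strength on all five meshes.
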(event `self.ReceiveBeginPlay`
  (`|ExecutionSequence`
    (:`then_0`
      (`KismetMaterialLibrary.CreateDynamicMaterialInstance` "/Game/Materials/Models/Enviroment/CrystalMat_Inst.CrystalMat_Inst"))
    (:`then_1`
      (`MeshComponent.SetVectorParameterValueOnMaterials` (`self.Crystal1`) "Emissive Color" (`KismetMathLibrary.Conv_LinearColorToVector` (`self.Color`)))
      (`MeshComponent.SetVectorParameterValueOnMaterials` (`self.Crystal2`) "Emissive Color" (`KismetMathLibrary.Conv_LinearColorToVector` (`self.Color`)))
      (`MeshComponent.SetVectorParameterValueOnMaterials` (`self.Crystal3`) "Emissive Color" (`KismetMathLibrary.Conv_LinearColorToVector` (`self.Color`)))
      (`MeshComponent.SetVectorParameterValueOnMaterials` (`self.Crystal4`) "Emissive Color" (`KismetMathLibrary.Conv_LinearColorToVector` (`self.Color`)))
      (`MeshComponent.SetVectorParameterValueOnMaterials` (`self.Sphere`) "Emissive Color" (`KismetMathLibrary.Conv_LinearColorToVector` (`self.Color`))))
    (:`then_2`
      (`LightComponent.SetLightColor` (`self.PointLight`) (`self.Color`) true))
    (:`then_3`
      (set `AudioComponent.Sound` (`self.SoundSlot`) (`self.Audio`) :!label _label))
    (:`then_4`
      (goto _label))))

(event `Activate`
  (`AudioComponent.Play` (`self.Audio`) 0.0)
  (bind (_direction _emissivestrength) (`Timeline|EmissionCycle` :!via `PlayFromStart`)
    (:`Update`
      (`MeshComponent.SetScalarParameterValueOnMaterials` (`self.Crystal1`) "Emissive Strength" _emissivestrength)
      (`MeshComponent.SetScalarParameterValueOnMaterials` (`self.Crystal2`) "Emissive Strength" _emissivestrength)
      (`MeshComponent.SetScalarParameterValueOnMaterials` (`self.Crystal3`) "Emissive Strength" _emissivestrength)
      (`MeshComponent.SetScalarParameterValueOnMaterials` (`self.Crystal4`) "Emissive Strength" _emissivestrength)
      (`MeshComponent.SetScalarParameterValueOnMaterials` (`self.Sphere`) "Emissive Strength" _emissivestrength))))

(fn `UserConstructionScript`)