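; Bird actor that flies once along a referenced spline path and stops at its end.
; BeginPlay snaps it to the first spline point and starts a looping timer that calls MoveBird instead of using Tick.
; Each call advances a fixed distance along the spline, applying location and only the yaw of its rotation.
; At the spline's length it clears the timer and sets IsFlying false on the BP_BirdAnimation instance.
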(event `self.ReceiveBeginPlay`
  (bind _spline (`/Game/Blueprints/BP_SplinePath.Spline` (`self.SplineRef`)))
  (`self.K2_SetActorLocationAndRotation` (`SplineComponent.GetLocationAtSplinePoint` _spline 0 "World") (`SplineComponent.GetRotationAtSplinePoint` _spline 0 "World"))
  (`KismetSystemLibrary.K2_SetTimer` null "MoveBird" 0.01 true))

(fn `MoveBird`
  (bind (_returnvalue_roll _returnvalue_pitch _returnvalue_yaw) (`KismetMathLibrary.BreakRotator` (`SplineComponent.GetRotationAtDistanceAlongSpline` (`/Game/Blueprints/BP_SplinePath.Spline` (`self.SplineRef`)) (`self.DistanceAlongSpline`) "World")))
  (bind (_returnvalue_x _returnvalue_y _returnvalue_z) (`KismetMathLibrary.BreakVector` (`SplineComponent.GetLocationAtDistanceAlongSpline` (`/Game/Blueprints/BP_SplinePath.Spline` (`self.SplineRef`)) (`self.DistanceAlongSpline`) "World")))
  (set `self.DistanceAlongSpline` (+ 2.0 (`self.DistanceAlongSpline`)))
  (`self.K2_SetActorLocationAndRotation` (`KismetMathLibrary.MakeVector` _returnvalue_x _returnvalue_y _returnvalue_z) (`KismetMathLibrary.MakeRotator` 0.0 0.0 _returnvalue_yaw))
  (if (>= (`self.DistanceAlongSpline`) (`/Game/Blueprints/BP_SplinePath.SplineLength` (`self.SplineRef`)))
    (`KismetSystemLibrary.K2_ClearTimer` null "MoveBird")
    (bind _asbp_bird_animation (cast `/Game/Blueprints/AnimationBlueprints/BP_BirdAnimation` (`SkeletalMeshComponent.GetAnimInstance` (`self.BirdMesh`))))
    (set `/Game/Blueprints/AnimationBlueprints/BP_BirdAnimation.IsFlying` false _asbp_bird_animation)))

(fn `UserConstructionScript`)