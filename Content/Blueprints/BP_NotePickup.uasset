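; BP_NotePickup is a spinning, color-tinted musical note pickup that plays the next sound in a shared sequence when collected.
; BeginPlay applies Color to the mesh's emissive parameter and starts a looping timer for BounceAndRotate, which only yaws the actor.
; PickUp plays the current NoteArray entry from BP_GameMode, activates particles and advances the shared index.
; It then hides the mesh and destroys the actor after a delay.
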(event `self.ReceiveBeginPlay`
  (`KismetSystemLibrary.K2_SetTimer` null "BounceAndRotate" 0.05 true)
  (`MeshComponent.SetVectorParameterValueOnMaterials` (`self.NoteMesh`) "Emissive Color" (`KismetMathLibrary.Conv_LinearColorToVector` (`self.Color`))))

(event `Pick Up`
  (bind _asbp_game_mode (cast `/Game/Blueprints/BP_GameMode` (`GameplayStatics.GetGameMode`)))
  (bind _notearrayhead (`/Game/Blueprints/BP_GameMode.NoteArrayHead` _asbp_game_mode))
  (`GameplayStatics.PlaySoundAtLocation` (`|GetArrayItem` (`/Game/Blueprints/BP_GameMode.NoteArray` _asbp_game_mode) _notearrayhead) (`self.K2_GetActorLocation`) (struct) 0.5 1.0 0.0 null null null)
  (`ActorComponent.Activate` (`self.ParticleEmitter`) false)
  (set `/Game/Blueprints/BP_GameMode.NoteArrayHead` (+ _notearrayhead 1) _asbp_game_mode)
  (`SceneComponent.SetVisibility` (`self.NoteMesh`) false false)
  (`KismetSystemLibrary.Delay` 10.0)
  (`self.K2_DestroyActor`))

(fn `BounceAndRotate`
  (`self.K2_AddActorLocalRotation` (`KismetMathLibrary.MakeRotator` 0.0 0.0 (`self.RotationSpeed`))))

(fn `UserConstructionScript`)