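; Box actor that changes color while a MotionControllerPawn overlaps its cube.
; BeginPlay creates a dynamic instance of M_Dynamic on the cube and enables player input.
; Overlap plays a timeline driving the Color parameter, stopping when the overlap ends and resuming on re-entry; completion activates the PSTransformationDone effect.
; A second timeline for the Glow parameter is never triggered.
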(event `self.ReceiveBeginPlay`
  (bind _returnvalue (`PrimitiveComponent.CreateDynamicMaterialInstance` (`self.Cube`) 0 "/Game/Materials/M_Dynamic.M_Dynamic" "None"))
  (`self.EnableInput` (`GameplayStatics.GetPlayerController` 0)))

(event `self.Cube.OnComponentBeginOverlap`
  (params (OverlappedComponent :type "PrimitiveComponent Object Reference") (OtherActor :type "Actor Object Reference") (OtherComp :type "PrimitiveComponent Object Reference") (OtherBodyIndex :type Integer) (bFromSweep :type Boolean) (SweepResult :type "HitResult Structure (by ref)"))
  (cast `/Game/Blueprints/MotionControllerPawn` OtherActor)
  (bind (_direction _color_fade) (`Timeline|Timeline_0` :!label _label)
    (:`Update`
      (`MaterialInstanceDynamic.SetVectorParameterValue` (stale `self.ReceiveBeginPlay` _returnvalue) "Color" _color_fade))
    (:`Finished`
      (`ActorComponent.Activate` (`self.PS_TransformationDone`) false))))

(event `self.Cube.OnComponentEndOverlap`
  (params (OverlappedComponent :type "PrimitiveComponent Object Reference") (OtherActor :type "Actor Object Reference") (OtherComp :type "PrimitiveComponent Object Reference") (OtherBodyIndex :type Integer))
  (cast `/Game/Blueprints/MotionControllerPawn` OtherActor)
  (goto _label :!via `Stop`))

(fn `UserConstructionScript`)