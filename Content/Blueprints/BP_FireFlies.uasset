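; BP_FireFlies is a firefly effect actor that switches its particle system on and off as the player's bear enters and leaves its Zone.
; Zone overlap events cast the other actor to BP_PathboundPlayer and respond only when the overlapping component is its BearCollision.
; Begin overlap activates ParticleSystem without a reset, and end overlap deactivates it.
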(event `self.Zone.OnComponentBeginOverlap`
  (params (OverlappedComponent :type "PrimitiveComponent Object Reference") (OtherActor :type "Actor Object Reference") (OtherComp :type "PrimitiveComponent Object Reference") (OtherBodyIndex :type Integer) (bFromSweep :type Boolean) (SweepResult :type "HitResult Structure (by ref)"))
  (bind _asbp_pathbound_player (cast `/Game/Blueprints/BP_PathboundPlayer` OtherActor))
  (if (== (`/Game/Blueprints/BP_PathboundPlayer.BearCollision` _asbp_pathbound_player) OtherComp)
    (`ActorComponent.Activate` (`self.ParticleSystem`) false)))

(event `self.Zone.OnComponentEndOverlap`
  (params (OverlappedComponent :type "PrimitiveComponent Object Reference") (OtherActor :type "Actor Object Reference") (OtherComp :type "PrimitiveComponent Object Reference") (OtherBodyIndex :type Integer))
  (bind _asbp_pathbound_player (cast `/Game/Blueprints/BP_PathboundPlayer` OtherActor))
  (if (== (`/Game/Blueprints/BP_PathboundPlayer.BearCollision` _asbp_pathbound_player) OtherComp)
    (`ActorComponent.Deactivate` (`self.ParticleSystem`))))

(fn `UserConstructionScript`)