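; BP_SoundKey is a playable musical key struck with VR motion controllers, labeled with its note name by the construction script.
; When a motion controller's NoteHitter component overlaps the Key, it plays the Note sound in 2D and rumbles that controller.
; The same hit restarts a timeline that animates the emissive strength of the four crystals in the referenced BP_CrystalCluster.
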(event `self.ReceiveBeginPlay`)

(event `self.ReceiveActorBeginOverlap`
  (params (OtherActor :type "Actor Object Reference")))

(event `self.Key.OnComponentBeginOverlap`
  (params (OverlappedComponent :type "PrimitiveComponent Object Reference") (OtherActor :type "Actor Object Reference") (OtherComp :type "PrimitiveComponent Object Reference") (OtherBodyIndex :type Integer) (bFromSweep :type Boolean) (SweepResult :type "HitResult Structure (by ref)"))
  (bind _asbp_motion_controller (cast `/Game/Blueprints/BP_MotionController` OtherActor))
  (if (== OtherComp (`/Game/Blueprints/BP_MotionController.NoteHitter` _asbp_motion_controller))
    (`|ExecutionSequence`
      (:`then_0`
        (`GameplayStatics.PlaySound2D` (`self.Note`) 1.0 1.0 0.0 null null)
        (`/Game/Blueprints/BP_MotionController.RumbleController` _asbp_motion_controller 0.1))
      (:`then_1`
        (bind _asbp_crystal_cluster (cast `/Game/Blueprints/BP_CrystalCluster` (`self.CrystalRef`)))
        (bind (_direction _emissive_strength) (`Timeline|Timeline_0` :!via `PlayFromStart`)
          (:`Update`
            (`MeshComponent.SetScalarParameterValueOnMaterials` (`/Game/Blueprints/BP_CrystalCluster.Crystal1` _asbp_crystal_cluster) "Emissive Strength" _emissive_strength)
            (`MeshComponent.SetScalarParameterValueOnMaterials` (`/Game/Blueprints/BP_CrystalCluster.Crystal2` _asbp_crystal_cluster) "Emissive Strength" _emissive_strength)
            (`MeshComponent.SetScalarParameterValueOnMaterials` (`/Game/Blueprints/BP_CrystalCluster.Crystal3` _asbp_crystal_cluster) "Emissive Strength" _emissive_strength)
            (`MeshComponent.SetScalarParameterValueOnMaterials` (`/Game/Blueprints/BP_CrystalCluster.Crystal4` _asbp_crystal_cluster) "Emissive Strength" _emissive_strength)))))))

(fn `UserConstructionScript`
  (`TextRenderComponent.K2_SetText` (`self.NoteText`) (`self.NoteName`)))