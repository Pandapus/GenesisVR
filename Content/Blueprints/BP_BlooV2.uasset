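; BP_BlooV2 is an actor that advances along a referenced spline whenever the player enters its proximity radius.
; It starts at spline point 1; each overlap jumps it forward by SpeedMultiplier in distance, with line traces setting its height.
; The overlap also flags it as moving for a fixed delay, then increments the point index.
; Tick eases rotation toward the next point's spline rotation while moving, otherwise toward the player.
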(event `self.ReceiveBeginPlay`
  (bind (_returnvalue_x _returnvalue_y) (`KismetMathLibrary.BreakVector` (`self.K2_GetActorLocation`)))
  (bind _returnvalue (`self.K2_GetActorLocation`))
  (bind (_returnvalue_x_2 _returnvalue_y_2) (`KismetMathLibrary.BreakVector` (`SplineComponent.GetLocationAtSplinePoint` (`/Game/Blueprints/BP_SplinePath.Spline` (`self.SplineRef`)) 1 "World")))
  (bind _outhit (`KismetSystemLibrary.LineTraceSingleForObjects` :`Start` _returnvalue :`End` (`KismetMathLibrary.MakeVector` _returnvalue_x _returnvalue_y -5000.0) :`ObjectTypes` (`|MakeArray` "ObjectTypeQuery7" :!type "EObjectTypeQuery Enum") :`DrawTime` 1.0))
  (`self.K2_SetActorLocationAndRotation` (`KismetMathLibrary.MakeVector` _returnvalue_x_2 _returnvalue_y_2 (.z (`.Location` (`GameplayStatics.BreakHitResult` _outhit)))) (`KismetMathLibrary.FindLookAtRotation` _returnvalue (`self.K2_GetActorLocation` (`self.PlayerRef`))))
  (set `self.CurrentSplinePoint` 1))

(event `self.ProximityRadius.OnComponentBeginOverlap`
  (params (OverlappedComponent :type "PrimitiveComponent Object Reference") (OtherActor :type "Actor Object Reference") (OtherComp :type "PrimitiveComponent Object Reference") (OtherBodyIndex :type Integer) (bFromSweep :type Boolean) (SweepResult :type "HitResult Structure (by ref)"))
  (bind (_returnvalue_x _returnvalue_y) (`KismetMathLibrary.BreakVector` (`self.K2_GetActorLocation`)))
  (bind (_returnvalue_x_2 _returnvalue_y_2) (`KismetMathLibrary.BreakVector` (`SplineComponent.GetLocationAtDistanceAlongSpline` (`/Game/Blueprints/BP_SplinePath.Spline` (`self.SplineRef`)) (`self.DistanceAlongSpline`) "World")))
  (if (== OtherActor (`self.PlayerRef`))
    (set `self.IsMoving` true)
    (set `self.DistanceAlongSpline` (+ (`self.SpeedMultiplier`) (`self.DistanceAlongSpline`)))
    (bind _outhit (`KismetSystemLibrary.LineTraceSingleForObjects` :`Start` (`KismetMathLibrary.MakeVector` _returnvalue_x _returnvalue_y 5000.0) :`End` (`KismetMathLibrary.MakeVector` _returnvalue_x _returnvalue_y -5000.0) :`ObjectTypes` (`|MakeArray` "ObjectTypeQuery7" :!type "EObjectTypeQuery Enum") :`DrawTime` 1.0))
    (`self.K2_SetActorLocationAndRotation` (`KismetMathLibrary.MakeVector` _returnvalue_x_2 _returnvalue_y_2 (.z (`.Location` (`GameplayStatics.BreakHitResult` _outhit)))))
    (`KismetSystemLibrary.Delay` 8.1)
    (set `self.CurrentSplinePoint` (+ (`self.CurrentSplinePoint`) 1))
    (set `self.IsMoving` false)))

(event `self.ReceiveTick`
  (params (DeltaSeconds :type "Float (single-precision)"))
  (if (`self.IsMoving`)
    (`self.K2_SetActorRotation` (`KismetMathLibrary.RLerp` (`self.K2_GetActorRotation`) (`SplineComponent.GetRotationAtSplinePoint` (`/Game/Blueprints/BP_SplinePath.Spline` (`self.SplineRef`)) (+ (`self.CurrentSplinePoint`) 1) "World") DeltaSeconds true))
    (else
      (`self.K2_SetActorRotation` (`KismetMathLibrary.RLerp` (`self.K2_GetActorRotation`) (`KismetMathLibrary.FindLookAtRotation` (`self.K2_GetActorLocation`) (`self.K2_GetActorLocation` (`self.PlayerRef`))) DeltaSeconds)))))

(fn `UserConstructionScript`)