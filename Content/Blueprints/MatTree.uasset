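; MatTree is an actor that changes the color of its static mesh when the BP_PathboundPlayer overlaps it.
; BeginPlay creates a dynamic M_Dynamic instance on material slot 1 and enables input, though no input events exist.
; Overlap begin plays a timeline driving the Color parameter; overlap end stops it in place without reversing.
; A second timeline for the Glow parameter is never triggered.
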(event `self.ReceiveBeginPlay`
  (bind _returnvalue (`PrimitiveComponent.CreateDynamicMaterialInstance` (`self.StaticMesh`) 1 "/Game/Materials/M_Dynamic.M_Dynamic" "None"))
  (`self.EnableInput` (`GameplayStatics.GetPlayerController` 0)))

(event `self.StaticMesh.OnComponentBeginOverlap`
  (params (OverlappedComponent :type "PrimitiveComponent Object Reference") (OtherActor :type "Actor Object Reference") (OtherComp :type "PrimitiveComponent Object Reference") (OtherBodyIndex :type Integer) (bFromSweep :type Boolean) (SweepResult :type "HitResult Structure (by ref)"))
  (cast `/Game/Blueprints/BP_PathboundPlayer` OtherActor)
  (bind (_direction _color_fade) (`Timeline|Timeline_0` :!label _label)
    (:`Update`
      (`MaterialInstanceDynamic.SetVectorParameterValue` (stale `self.ReceiveBeginPlay` _returnvalue) "Color" _color_fade))))

(event `self.StaticMesh.OnComponentEndOverlap`
  (params (OverlappedComponent :type "PrimitiveComponent Object Reference") (OtherActor :type "Actor Object Reference") (OtherComp :type "PrimitiveComponent Object Reference") (OtherBodyIndex :type Integer))
  (cast `/Game/Blueprints/BP_PathboundPlayer` OtherActor)
  (goto _label :!via `Stop`))

(fn `UserConstructionScript`)