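; BP_FireWorks is an actor that sets off a particle effect when the player's LookAtBox overlaps its TriggerSphere.
; The overlap handler accepts only that component of BP_PathboundPlayer, so other parts of the player do not trigger it.
; The effect activates only while EnablerRef is Enabled, and the actor destroys itself after a fixed delay.
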(event `self.TriggerSphere.OnComponentBeginOverlap`
  (params (OverlappedComponent :type "PrimitiveComponent Object Reference") (OtherActor :type "Actor Object Reference") (OtherComp :type "PrimitiveComponent Object Reference") (OtherBodyIndex :type Integer) (bFromSweep :type Boolean) (SweepResult :type "HitResult Structure (by ref)"))
  (bind _asbp_pathbound_player (cast `/Game/Blueprints/BP_PathboundPlayer` OtherActor))
  (if (== (`/Game/Blueprints/BP_PathboundPlayer.LookAtBox` _asbp_pathbound_player) OtherComp)
    (if (`/Game/Blueprints/BP_FireworksEnabler.Enabled` (`self.EnablerRef`))
      (`ActorComponent.Activate` (`self.ParticleEmitter`) false)
      (`KismetSystemLibrary.Delay` 10.0)
      (`self.K2_DestroyActor`))))

(fn `UserConstructionScript`)