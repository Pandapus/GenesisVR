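; Bloo is an actor that advances along a referenced spline point by point whenever the player's bear collision enters its proximity radius.
; Each trigger disables the radius and plays the MoveTime timeline, whose Finished event re-enables it and sets location from a lerp between points.
; A downward object trace supplies height.
; Tick smoothly yaws Bloo toward the next point while moving, otherwise toward the player.
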(event `self.ReceiveBeginPlay`
  (bind (_returnvalue_x _returnvalue_y) (`KismetMathLibrary.BreakVector` (`self.K2_GetActorLocation`)))
  (bind _returnvalue (`self.K2_GetActorLocation`))
  (bind (_returnvalue_x_2 _returnvalue_y_2) (`KismetMathLibrary.BreakVector` (`SplineComponent.GetLocationAtSplinePoint` (`/Game/Blueprints/BP_SplinePath.Spline` (`self.SplineRef`)) 1 "World")))
  ;[1 1 1] Set initial position and rotation
  (bind _z_value (`self.GetZValue` _returnvalue (`KismetMathLibrary.MakeVector` _returnvalue_x _returnvalue_y -5000.0)))
  (`self.K2_SetActorLocationAndRotation` (`KismetMathLibrary.MakeVector` _returnvalue_x_2 _returnvalue_y_2 _z_value) (`KismetMathLibrary.FindLookAtRotation` _returnvalue (`self.K2_GetActorLocation` (`self.PlayerRef`))))
  (set `self.CurrentSplinePoint` 1))

(event `self.ProximityRadius.OnComponentBeginOverlap`
  (params (OverlappedComponent :type "PrimitiveComponent Object Reference") (OtherActor :type "Actor Object Reference") (OtherComp :type "PrimitiveComponent Object Reference") (OtherBodyIndex :type Integer) (bFromSweep :type Boolean) (SweepResult :type "HitResult Structure (by ref)"))
  ;[1 1 1] Pick new location and walk there when player gets close
  (if (== OtherComp (`/Game/Blueprints/BP_PathboundPlayer.BearCollision` (`self.PlayerRef`)))
    (set `self.IsMoving` true)
    (`PrimitiveComponent.SetCollisionEnabled` (`self.ProximityRadius`) "NoCollision")
    (set `self.CurrentSplinePoint` (+ (`self.CurrentSplinePoint`) 1))
    (bind (_direction _movealpha) (`Timeline|MoveTime` :!via `PlayFromStart`)
      (:`Finished`
        (set `self.IsMoving` false)
        (`PrimitiveComponent.SetCollisionEnabled` (`self.ProximityRadius`) "QueryOnly")
        (bind (_returnvalue_x _returnvalue_y) (`KismetMathLibrary.BreakVector` (`KismetMathLibrary.VLerp` (`SplineComponent.GetLocationAtSplinePoint` (`/Game/Blueprints/BP_SplinePath.Spline` (`self.SplineRef`)) (- (`self.CurrentSplinePoint`) 1) "World") (`SplineComponent.GetLocationAtSplinePoint` (`/Game/Blueprints/BP_SplinePath.Spline` (`self.SplineRef`)) (`self.CurrentSplinePoint`) "World") _movealpha)))
        (bind _z_value (`self.GetZValue` (`KismetMathLibrary.MakeVector` _returnvalue_x _returnvalue_y 5000.0) (`KismetMathLibrary.MakeVector` _returnvalue_x _returnvalue_y -5000.0)))
        (`self.K2_SetActorLocation` (`KismetMathLibrary.MakeVector` _returnvalue_x _returnvalue_y _z_value))))))

(event `self.ReceiveTick`
  (params (DeltaSeconds :type "Float (single-precision)"))
  (bind _returnvalue (* (`self.TurnMultiplier`) DeltaSeconds))
  (bind (_returnvalue_roll _returnvalue_pitch _returnvalue_yaw) (`KismetMathLibrary.BreakRotator` (`KismetMathLibrary.RLerp` (`self.K2_GetActorRotation`) (`KismetMathLibrary.FindLookAtRotation` (`self.K2_GetActorLocation`) (`self.K2_GetActorLocation` (`self.PlayerRef`))) _returnvalue true)))
  (bind (_returnvalue_roll_2 _returnvalue_pitch_2 _returnvalue_yaw_2) (`KismetMathLibrary.BreakRotator` (`KismetMathLibrary.RLerp` (`self.K2_GetActorRotation`) (`KismetMathLibrary.FindLookAtRotation` (`self.K2_GetActorLocation`) (`SplineComponent.GetLocationAtSplinePoint` (`/Game/Blueprints/BP_SplinePath.Spline` (`self.SplineRef`)) (`self.CurrentSplinePoint`) "World")) _returnvalue true)))
  ;[1 1 1] Look at direction (player when not walking, next point when walking)
  (if (`self.IsMoving`)
    (`self.K2_SetActorRotation` (`KismetMathLibrary.MakeRotator` 0.0 0.0 _returnvalue_yaw_2))
    (else
      (`self.K2_SetActorRotation` (`KismetMathLibrary.MakeRotator` 0.0 0.0 _returnvalue_yaw)))))

(fn `GetZValue`
  (params (Start :type "Vector Structure") (End :type "Vector Structure"))
  (returns (`Z-Value` :type "Float (double-precision)"))
  (bind _outhit (`KismetSystemLibrary.LineTraceSingleForObjects` :`Start` Start :`End` End :`ObjectTypes` (`|MakeArray` "ObjectTypeQuery7" :!type "EObjectTypeQuery Enum") :`DrawTime` 1.0))
  (return (.z (`.Location` (`GameplayStatics.BreakHitResult` _outhit)))))

(fn `UserConstructionScript`)