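; Procedural hat actor that assembles a random hat from top, base and ornament meshes on BeginPlay.
; Each part draws a mesh from its own list, then top and base get a fabric material and the ornament gets metal.
; Random U tiling on all parts and V tiling on the fabric parts add variation.
; The Construction Script holds a disconnected, similar copy of this logic, so randomization happens only at runtime.
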(event `self.ReceiveBeginPlay`
  (bind _array (`|MakeArray` "/Game/Models/Meshes/M__OrnOctagon.M__OrnOctagon" "/Game/Models/Meshes/M__OrnTriangle.M__OrnTriangle" :!type "StaticMesh Object Reference"))
  (bind _array_2 (`|MakeArray` "/Game/Models/Meshes/M__TopHatCurve.M__TopHatCurve" "/Game/Models/Meshes/M__TopBowler.M__TopBowler" "/Game/Models/Meshes/M_TopCone.M_TopCone" :!type "StaticMesh Object Reference"))
  (bind _array_3 (`|MakeArray` "/Game/Models/Meshes/M__BaseCylinder.M__BaseCylinder" "/Game/Models/Meshes/M__BaseRound.M__BaseRound" :!type "StaticMesh Object Reference"))
  (bind _array_4 (`|MakeArray` (`self.TopMesh`) (`self.BaseMesh`) :!type "MeshComponent Object Reference"))
  (`|ExecutionSequence`
    (:`then_0`
      (`StaticMeshComponent.SetStaticMesh` (`self.TopMesh`) (`|GetArrayItem` _array_2 (`KismetMathLibrary.RandomInteger` (`KismetArrayLibrary.Array_Length` _array_2))))
      (`StaticMeshComponent.SetStaticMesh` (`self.BaseMesh`) (`|GetArrayItem` _array_3 (`KismetMathLibrary.RandomInteger` (`KismetArrayLibrary.Array_Length` _array_3))))
      (`StaticMeshComponent.SetStaticMesh` (`self.OrnateMesh`) (`|GetArrayItem` _array (`KismetMathLibrary.RandomInteger` (`KismetArrayLibrary.Array_Length` _array)))))
    (:`then_1`
      (`PrimitiveComponent.SetMaterial` (`self.TopMesh`) 0 "/Game/Materials/Models/Mat_Fabric.Mat_Fabric")
      (`PrimitiveComponent.SetMaterial` (`self.BaseMesh`) 0 "/Game/Materials/Models/Mat_Fabric.Mat_Fabric")
      (`PrimitiveComponent.SetMaterial` (`self.OrnateMesh`) 0 "/Game/Materials/Models/Mat_Metal.Mat_Metal")
      (`MeshComponent.SetScalarParameterValueOnMaterials` (`self.OrnateMesh`) "U Tile" (* (`KismetMathLibrary.RandomInteger` 3) 0.3))
      (for _array_element _array_4
        (`MeshComponent.SetScalarParameterValueOnMaterials` _array_element "U Tile" (* (`KismetMathLibrary.RandomInteger` 5) 0.2))
        (`MeshComponent.SetScalarParameterValueOnMaterials` _array_4 "V Tile" (* (`KismetMathLibrary.RandomInteger` 3) 0.2))))))

(fn `UserConstructionScript`)